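; Team artifact for a team game mode: its own team can carry it, and enemy damage destroys it, notifying TW_GameState.
; Server-side trigger overlaps offer pickup to teammates, then the artifact attaches to the carrier's neck socket.
; It drops at the carrier's death location or onto ground traced ahead of them, and can be locked against pickup.
; RepNotifies apply team colors, toggle the trigger, and reveal the beam to teammates or everyone.
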(event OnComponentBeginOverlap(TriggerSphere)
  (params (OtherActor :type Actor%20Object%20Reference) (OtherComp :type Primitive%20Component%20Object%20Reference) (OtherBodyIndex :type Integer) (bFromSweep :type Boolean) (SweepResult :type Hit%20Result%20Structure%20%28by%20ref%29))
  (Networking|SwitchHasAuthority
    (:Authority
      (bind _astw_playerpawntest_c (Utilities|Casting|CastToTW_PlayerPawnTest OtherActor))
      (if (Math|Boolean|ANDBoolean (== (Variables|Default|GetTeamID) (Variables|/Script/Engine.Actor|GetTargetingTeam _astw_playerpawntest_c)) (not (Variables|Default|GetGotPickedUp)) (Variables|Default|GetCanBePickedUp))
        (Default|EnteredArtifactTrigger _astw_playerpawntest_c self)))))

(event OnComponentEndOverlap(TriggerSphere)
  (params (OtherActor :type Actor%20Object%20Reference) (OtherComp :type Primitive%20Component%20Object%20Reference) (OtherBodyIndex :type Integer))
  (Networking|SwitchHasAuthority
    (:Authority
      (bind _astw_playerpawntest_c (Utilities|Casting|CastToTW_PlayerPawnTest OtherActor))
      (Default|LeftArtifactTrigger _astw_playerpawntest_c self))))

(event Custom|SetTeam
  (params (Team :type TW_Team_Enum%20Enum :default "NewEnumerator0"))
  (Variables|Default|SetTeam Team)
  (switch Utilities|FlowControl|Switch|SwitchonTW_Team_Enum Team
    (:NewEnumerator0
      (bind _astw_gamestate_c (Utilities|Casting|CastToTW_GameState (Game|GetGameState)))
      (Variables|Default|SetTeamID (Variables|/Game/Mods/TribeWars/TW_GameState.TW_GameState_C|GetRedTeamID _astw_gamestate_c)))
    (:NewEnumerator1
      (bind _astw_gamestate_c_2 (Utilities|Casting|CastToTW_GameState (Game|GetGameState)))
      (Variables|Default|SetTeamID (Variables|/Game/Mods/TribeWars/TW_GameState.TW_GameState_C|GetBlueTeamID _astw_gamestate_c_2))))
  (Variables|Default|SetIsVisibleForFriendlyTeam true)
  (Networking|ForceNetUpdate))

(event Custom|TryToPickupArtifact
  (params (Carrier :type Actor%20Object%20Reference))
  (bind _astw_playerpawntest_c (Utilities|Casting|CastToTW_PlayerPawnTest Carrier))
  (if (not (Variables|Default|GetGotPickedUp))
    (Variables|Default|SetGotPickedUp true)
    (Variables|Default|SetCarrier _astw_playerpawntest_c)
    (CallFunction|AttachtoPlayer)
    (Networking|ForceNetUpdate)
    (Default|BacameCarrier (Variables|Default|GetCarrier) self)
    (EventDispatchers|BindEventtoOnDied (Variables|Default|GetCarrier) (delegate Custom|PrimalCharacterDied__DelegateSignature_Event))))

(event Custom|RevealFlagForEveryone
  (Variables|Default|SetIsVisibleForAll true)
  (Networking|ForceNetUpdate))

(event Custom|DropArtifact
  (params (CarrierDied :type Boolean) (DeathLocation :type Vector))
  (Variables|Default|SetGotPickedUp false)
  (CallFunction|DetachfromPlayer CarrierDied DeathLocation)
  (Networking|ForceNetUpdate)
  (EventDispatchers|UnbindallEventsfromOnDied (Variables|Default|GetCarrier))
  (Variables|Default|SetCarrier 0))

(event Custom|PrimalCharacterDied__DelegateSignature_Event
  (params (DiedCharacter :type Primal%20Character%20Object%20Reference))
  (if (== (Variables|/Script/Engine.Actor|GetTargetingTeam DiedCharacter) (Variables|Default|GetTeamID))
    (CallFunction|DropArtifact true (Transformation|GetActorLocation DiedCharacter))))

(event Custom|DisableArtifactMovability
  (Variables|Default|SetCanBePickedUp false)
  (Default|ForceDroptheArtifact (Variables|Default|GetCarrier) self))

(event EventAnyDamage
  (params (Damage :type Float%20%28single-precision%29) (DamageType :type Damage%20Type%20Object%20Reference) (InstigatedBy :type Controller%20Object%20Reference) (DamageCauser :type Actor%20Object%20Reference))
  (bind _astw_gamestate_c (Utilities|Casting|CastToTW_GameState (Game|GetGameState)))
  (if (and (Variables|/Game/Mods/TribeWars/TW_GameState.TW_GameState_C|GetGameRunningState _astw_gamestate_c) (!= (Variables|/Script/Engine.Actor|GetTargetingTeam InstigatedBy) (Variables|Default|GetTeamID)))
    (Variables|Default|SetDamageDone (+ Damage (Variables|Default|GetDamageDone)))
    (if (>= (Variables|Default|GetDamageDone) (Variables|Default|GetHealth))
      (Utilities|FlowControl|DoOnce false
        (:Completed
          (bind _astw_gamestate_c_2 (Utilities|Casting|CastToTW_GameState (Game|GetGameState)))
          (Default|ArtifactGotDestroyed _astw_gamestate_c_2 (Variables|Default|GetTeamID)))))))

(event Input|KeyboardEvents|ShiftE
  (:Pressed
    (bind _astw_playerpawntest_c (Utilities|Casting|CastToTW_PlayerPawnTest (Game|Player|GetPlayerPawn 0)))
    (Default|ShiftEGotClicked _astw_playerpawntest_c self)))

(fn ConstructionScript
  (bind _staticmesh1 (Variables|Default|GetStaticMesh1))
  (Utilities|FlowControl|Sequence
    (:then_0
      (bind _returnvalue (Rendering|Material|CreateDynamicMaterialInstance (Variables|Default|GetBeam) 0 "/Game/Mods/TribeWars/Materials/TW_ArtifactBeam_Mat_Inst.TW_ArtifactBeam_Mat_Inst" :!class /Script/Engine.PrimitiveComponent))
      (Variables|Default|SetBeamMaterial _returnvalue))
    (:then_1
      (bind _returnvalue_2 (Rendering|Material|CreateDynamicMaterialInstance _staticmesh1 0 (Utilities|Array|Get(acopy) (Variables|/Script/Engine.MeshComponent|GetMaterials _staticmesh1)) :!class /Script/Engine.PrimitiveComponent))
      (Variables|Default|SetArtifactMaterial _returnvalue_2))))

(fn AttachtoPlayer
  (bind _carrier (Variables|Default|GetCarrier))
  (bind _mesh (Variables|/Script/Engine.Character|GetMesh _carrier))
  (Class|Actor|AttachRootComponentto _mesh "Cnt_Neck_Joint001_JNT_SKL" "SnapToTarget" true)
  (Transformation|SetActorRelativeLocation "0.000000,70.000000,-25.000000")
  (Transformation|SetActorRotation (Transformation|GetWorldRotation _mesh))
  (Transformation|AddActorLocalRotation "0,-90.000000, 0" false)
  (Transformation|AddActorLocalRotation "0.000000,0.000000,5.000000" false)
  (Transformation|SetActorScale3D (Math|Vector|MakeVector 1.0 1.0 1.0)))

(fn OnRepTeamID)

(fn OnRepGotPickedUp
  (Variables|/Script/Engine.PrimitiveComponent|SetbGenerateOverlapEvents (Variables|Default|GetTriggerSphere) (not (Variables|Default|GetGotPickedUp)))
  (bind _astw_playerpawntest_c (Utilities|Casting|CastToTW_PlayerPawnTest (Game|Player|GetPlayerPawn 0)))
  (Default|DisablePickupPromptforNonCarrier _astw_playerpawntest_c))

(fn DetachfromPlayer
  (params (CarrierDied :type Boolean) (DeathLocation :type Vector))
  (bind _carrier (Variables|Default|GetCarrier))
  (bind _triggersphere (Variables|Default|GetTriggerSphere))
  (bind _mesh (Variables|/Script/Engine.Character|GetMesh _carrier))
  (bind _sphereradius (Variables|/Script/Engine.SphereComponent|GetSphereRadius _triggersphere))
  (bind _returnvalue (Math|Vector|GetForwardVector _mesh))
  (bind _returnvalue_2 (Transformation|GetWorldLocation _mesh))
  (bind _returnvalue_3 (* _sphereradius 1.5))
  (bind _returnvalue_4 (* _returnvalue _returnvalue_3))
  (bind _returnvalue_5 (+ _returnvalue_2 _returnvalue_4))
  (bind (_x _y _z) (Math|Vector|BreakVector _returnvalue_5))
  (Class|Actor|DetachRootComponentfromParent true)
  (if CarrierDied
    (Transformation|SetActorLocationAndRotation DeathLocation "0, 0, 0")
    (else
      (bind (_outhit _returnvalue_6) (Collision|LineTraceByChannel (Math|Vector|MakeVector _x _y (+ _z 5e+02)) (Math|Vector|MakeVector _x _y (+ _z -4e+03)) "ECC_WorldStatic" false 0 "None"))
      (if _returnvalue_6
        (Transformation|SetActorLocationAndRotation (.Location (Collision|BreakHitResult _outhit)) "0, 0, 0")
        (else
          (Transformation|SetActorLocationAndRotation _returnvalue_2 "0, 0, 0"))))))

(fn OnRepIsVisibleforFriendlyTeam
  (if (not (Networking|IsDedicatedServer))
    (if (== (Variables|/Script/Engine.Actor|GetTargetingTeam (Game|GetPlayerController 0)) (Variables|Default|GetTeamID))
      (Development|SetHiddeninGame (Variables|Default|GetBeam) false false))))

(fn OnRepIsVisibleforAll
  (Development|SetHiddeninGame (Variables|Default|GetBeam) false false))

(fn OnRepTeam
  (bind _artifactmaterial (Variables|Default|GetArtifactMaterial))
  (bind _artifactmaterial_2 (Variables|Default|GetArtifactMaterial))
  (switch Utilities|FlowControl|Switch|SwitchonTW_Team_Enum (Variables|Default|GetTeam)
    (:NewEnumerator0
      (Rendering|Material|SetVectorParameterValue (Variables|Default|GetBeamMaterial) "Color" "(R=1.000000,G=0.000000,B=0.000000,A=1.000000)" :!class /Script/Engine.MaterialInstanceDynamic)
      (Rendering|Material|SetVectorParameterValue _artifactmaterial "Color0" "(R=1.000000,G=0.000000,B=0.000000,A=1.000000)" :!class /Script/Engine.MaterialInstanceDynamic)
      (Rendering|Material|SetVectorParameterValue _artifactmaterial "Color1" "(R=1.000000,G=0.000000,B=0.000000,A=1.000000)" :!class /Script/Engine.MaterialInstanceDynamic)
      (Rendering|Material|SetVectorParameterValue _artifactmaterial "Color2" "(R=1.000000,G=0.000000,B=0.000000,A=1.000000)" :!class /Script/Engine.MaterialInstanceDynamic)
      (Rendering|Material|SetVectorParameterValue _artifactmaterial "Color3" "(R=1.000000,G=0.000000,B=0.000000,A=1.000000)" :!class /Script/Engine.MaterialInstanceDynamic)
      (Rendering|Material|SetVectorParameterValue _artifactmaterial "Color4" "(R=1.000000,G=0.000000,B=0.000000,A=1.000000)" :!class /Script/Engine.MaterialInstanceDynamic)
      (Rendering|Material|SetVectorParameterValue _artifactmaterial "Color5" "(R=1.000000,G=0.000000,B=0.000000,A=1.000000)" :!class /Script/Engine.MaterialInstanceDynamic))
    (:NewEnumerator1
      (Rendering|Material|SetVectorParameterValue (Variables|Default|GetBeamMaterial) "Color" "(R=0.000000,G=0.000000,B=1.000000,A=1.000000)" :!class /Script/Engine.MaterialInstanceDynamic)
      (Rendering|Material|SetVectorParameterValue _artifactmaterial_2 "Color0" "(R=0.000000,G=0.000000,B=1.000000,A=1.000000)" :!class /Script/Engine.MaterialInstanceDynamic)
      (Rendering|Material|SetVectorParameterValue _artifactmaterial_2 "Color1" "(R=0.000000,G=0.000000,B=1.000000,A=1.000000)" :!class /Script/Engine.MaterialInstanceDynamic)
      (Rendering|Material|SetVectorParameterValue _artifactmaterial_2 "Color2" "(R=0.000000,G=0.000000,B=1.000000,A=1.000000)" :!class /Script/Engine.MaterialInstanceDynamic)
      (Rendering|Material|SetVectorParameterValue _artifactmaterial_2 "Color3" "(R=0.000000,G=0.000000,B=1.000000,A=1.000000)" :!class /Script/Engine.MaterialInstanceDynamic)
      (Rendering|Material|SetVectorParameterValue _artifactmaterial_2 "Color4" "(R=0.000000,G=0.000000,B=1.000000,A=1.000000)" :!class /Script/Engine.MaterialInstanceDynamic)
      (Rendering|Material|SetVectorParameterValue _artifactmaterial_2 "Color5" "(R=0.000000,G=0.000000,B=1.000000,A=1.000000)" :!class /Script/Engine.MaterialInstanceDynamic))))