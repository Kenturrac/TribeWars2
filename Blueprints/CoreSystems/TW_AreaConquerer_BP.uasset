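; Capturable team area that Red and Blue players contest by standing inside a sphere trigger.
; Each second it compares living players per team, moving progress by the capped majority, draining the rival's first and resetting when empty.
; At 100 the server locks the area, hands structures gathered within the radius at startup to the winners and scores their capturers.
; UpdateScore also refreshes the local player's capture widget on clients.
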(event OnComponentBeginOverlap(trigger)
  (params (OtherActor :type Actor%20Object%20Reference) (OtherComp :type Primitive%20Component%20Object%20Reference) (OtherBodyIndex :type Integer) (bFromSweep :type Boolean) (SweepResult :type Hit%20Result%20Structure%20%28by%20ref%29))
  (bind _capturingplayercontrollers (Variables|Default|GetCapturingPlayerControllers))
  (bind _asplayerpawntest_c (Utilities|Casting|CastToPlayerPawnTest OtherActor))
  (if (Variables|Default|GetCanBeCaptured)
    (Utilities|TWDedicatedServerCheck
      (:Yes
        (bind _astw_playercontrollerblueprint_c (Utilities|Casting|CastToTW_PlayerControllerBlueprint (Pawn|GetController _asplayerpawntest_c)))
        (if (Utilities|Array|ContainsItem _capturingplayercontrollers _astw_playercontrollerblueprint_c)
          _
          (else
            (Utilities|Array|Add _capturingplayercontrollers _astw_playercontrollerblueprint_c)))
        (if (not (Variables|Default|GetIsProgressing))
          (Variables|Default|SetIsProgressing true)
          (CallFunction|CheckforProgress)))
      (:No
        (if (Pawn|IsLocallyControlled _asplayerpawntest_c)
          (Utilities|IsValid (Variables|Default|GetCaptureWidget)
            (:Is%20Not%20Valid
              (bind _returnvalue (UserInterface|CreateWidget "/Game/Mods/TribeWars/HUD/TW_CaptureArea_Widget.TW_CaptureArea_Widget_C" (Game|GetPlayerController 0)))
              (Variables|Default|SetCaptureWidget _returnvalue)
              (UserInterface|Viewport|AddtoViewport _returnvalue)
              (Default|UpdateWidget _returnvalue (Variables|Default|GetOwningTeam) (Variables|Default|GetScoringTeam) (Variables|Default|GetProgress)))))))))

(event OnComponentEndOverlap(trigger)
  (params (OtherActor :type Actor%20Object%20Reference) (OtherComp :type Primitive%20Component%20Object%20Reference) (OtherBodyIndex :type Integer))
  (bind _astw_playerpawntest_c (Utilities|Casting|CastToTW_PlayerPawnTest OtherActor))
  (if (Pawn|IsLocallyControlled _astw_playerpawntest_c)
    (Utilities|IsValid (Variables|Default|GetCaptureWidget)
      (:Is%20Valid
        (Class|UserWidget|RemovefromViewport (Variables|Default|GetCaptureWidget))
        (Variables|Default|SetCaptureWidget 0)))))

(event Custom|CheckForProgress
  (bind _trigger (Variables|Default|Gettrigger))
  (bind _overlappingactors (Collision|GetOverlappingActors _trigger "/Game/PrimalEarth/CoreBlueprints/PlayerPawnTest.PlayerPawnTest_C" :!class /Script/Engine.PrimitiveComponent))
  (Variables|Default|SetRedTeamInArea 0)
  (Variables|Default|SetBlueTeamInArea 0)
  (if (and (> (Utilities|Array|Length _overlappingactors) 0) (< (Variables|Default|GetProgress) 100))
    (Utilities|Time|SetTimerbyFunctionName 0 "CheckForProgress" 1.0)
    (bind _astw_gamestate_c (Utilities|Casting|CastToTW_GameState (Game|GetGameState)))
    (for _array_element _overlappingactors
      (bind _asplayerpawntest_c (Utilities|Casting|CastToPlayerPawnTest _array_element))
      (if (Class|PrimalCharacter|IsAlive _asplayerpawntest_c)
        (if (== (Variables|/Script/Engine.Actor|GetTargetingTeam _array_element) (Variables|/Game/Mods/TribeWars/TW_GameState.TW_GameState_C|GetRedTeamID _astw_gamestate_c))
          (Variables|Default|SetRedTeamInArea (+ (Variables|Default|GetRedTeamInArea) 1))
          (elif (== (Variables|/Script/Engine.Actor|GetTargetingTeam _array_element) (Variables|/Game/Mods/TribeWars/TW_GameState.TW_GameState_C|GetBlueTeamID _astw_gamestate_c))
            (Variables|Default|SetBlueTeamInArea (+ (Variables|Default|GetBlueTeamInArea) 1))))))
    (Math|Integer|CompareInt (Variables|Default|GetRedTeamInArea) (Variables|Default|GetBlueTeamInArea)
      (:>
        (CallFunction|CalculateProgress "NewEnumerator0"))
      (:==
        (CallFunction|CalculateProgress "NewEnumerator2"))
      (:<
        (CallFunction|CalculateProgress "NewEnumerator1")))
    (else
      (Variables|Default|SetIsProgressing false)
      (Utilities|Array|Clear (Variables|Default|GetCapturingPlayerControllers))
      (Variables|Default|SetProgress 0)
      (Variables|Default|SetOwningTeam "NewEnumerator2")
      (Variables|Default|SetScoringTeam "NewEnumerator2"))))

(event Custom|UpdateScore
  (params (OwningTeam :type TW_Team_Enum%20Enum :default "NewEnumerator2") (ScoringTeam :type TW_Team_Enum%20Enum :default "NewEnumerator2") (Progress :type Integer))
  (bind _capturewidget (Variables|Default|GetCaptureWidget))
  (Utilities|TWDedicatedServerCheck
    (:Yes
      (if (== Progress 100)
        (Utilities|FlowControl|DoOnce false
          (:Completed
            (switch Utilities|FlowControl|Switch|SwitchonTW_Team_Enum OwningTeam
              (:NewEnumerator0
                (bind _astw_gamestate_c (Utilities|Casting|CastToTW_GameState (Game|GetGameState)))
                (for _array_element (Variables|Default|GetStructureArray)
                  (Variables|/Script/Engine.Actor|SetTargetingTeam _array_element (Variables|/Game/Mods/TribeWars/TW_GameState.TW_GameState_C|GetRedTeamID _astw_gamestate_c)))
                (Variables|Default|SetCanBeCaptured false)
                (Networking|ForceNetUpdate)
                (for _array_element_2 (Variables|Default|GetCapturingPlayerControllers)
                  (if (== (Variables|/Script/Engine.Actor|GetTargetingTeam _array_element_2) (Variables|/Game/Mods/TribeWars/TW_GameState.TW_GameState_C|GetRedTeamID _astw_gamestate_c))
                    (Default|CalculateScoreUpdate _astw_gamestate_c _array_element_2 "NewEnumerator8"))))
              (:NewEnumerator1
                (bind _astw_gamestate_c_2 (Utilities|Casting|CastToTW_GameState (Game|GetGameState)))
                (for _array_element_3 (Variables|Default|GetStructureArray)
                  (Variables|/Script/Engine.Actor|SetTargetingTeam _array_element_3 (Variables|/Game/Mods/TribeWars/TW_GameState.TW_GameState_C|GetBlueTeamID _astw_gamestate_c_2)))
                (Variables|Default|SetCanBeCaptured false)
                (Networking|ForceNetUpdate)
                (for _array_element_4 (Variables|Default|GetCapturingPlayerControllers)
                  (if (== (Variables|/Script/Engine.Actor|GetTargetingTeam _array_element_4) (Variables|/Game/Mods/TribeWars/TW_GameState.TW_GameState_C|GetBlueTeamID _astw_gamestate_c_2))
                    (Default|CalculateScoreUpdate _astw_gamestate_c_2 _array_element_4 "NewEnumerator8")))))))))
    (:No
      (Variables|Default|SetOwningTeam OwningTeam)
      (Variables|Default|SetScoringTeam ScoringTeam)
      (Variables|Default|SetProgress Progress)
      (Utilities|IsValid _capturewidget
        (:Is%20Valid
          (Default|UpdateWidget _capturewidget OwningTeam ScoringTeam Progress))))))

(event EventBeginPlay
  (Utilities|FlowControl|Delay (Math|Random|RandomFloatinRange 2.0 5.0))
  (Utilities|TWDedicatedServerCheck
    (:Yes
      (bind _outactors (Actor|GetAllActorsOfClass "/Script/ShooterGame.PrimalStructure"))
      (for _array_element _outactors
        (bind _returnvalue (Transformation|GetDistanceTo _array_element self))
        (if (<= _returnvalue (Variables|Default|GetRadius))
          (Utilities|Array|Add (Variables|Default|GetStructureArray) _array_element)))
      (Variables|Default|SetCanBeCaptured true)
      (Networking|ForceNetUpdate))))

(fn ConstructionScript
  (Components|Sphere|SetSphereRadius (Variables|Default|Gettrigger) (Variables|Default|GetRadius) true)
  (if (Variables|Default|GetIsDebug)
    (Development|SetHiddeninGame (Variables|Default|Gettrigger) (not (Variables|Default|GetIsDebug)) false)))

(fn CalculateProgress
  (params (ScoringTeam :type TW_Team_Enum%20Enum :default "NewEnumerator2"))
  (bind _blueteaminarea (Variables|Default|GetBlueTeamInArea))
  (bind _redteaminarea (Variables|Default|GetRedTeamInArea))
  (bind _blueteaminarea_2 (Variables|Default|GetBlueTeamInArea))
  (bind _redteaminarea_2 (Variables|Default|GetRedTeamInArea))
  (bind _blueteaminarea_3 (Variables|Default|GetBlueTeamInArea))
  (bind _redteaminarea_3 (Variables|Default|GetRedTeamInArea))
  (bind _blueteaminarea_4 (Variables|Default|GetBlueTeamInArea))
  (bind _redteaminarea_4 (Variables|Default|GetRedTeamInArea))
  (bind _returnvalue (- _redteaminarea_2 _blueteaminarea))
  (bind _returnvalue_2 (- _redteaminarea _blueteaminarea_2))
  (bind _returnvalue_3 (- _blueteaminarea_3 _redteaminarea_3))
  (bind _returnvalue_4 (- _blueteaminarea_4 _redteaminarea_4))
  (Variables|Default|SetScoringTeam ScoringTeam)
  (switch Utilities|FlowControl|Switch|SwitchonTW_Team_Enum ScoringTeam
    (:NewEnumerator2
      (CallFunction|UpdateScore (Variables|Default|GetOwningTeam) (Variables|Default|GetScoringTeam) (Variables|Default|GetProgress) :!label _label))
    (:NewEnumerator0
      (if (Utilities|Enum|Equal(Enum) (Variables|Default|GetOwningTeam) "NewEnumerator2") :!label _label_2
        (switch Utilities|FlowControl|Switch|SwitchonTW_Team_Enum ScoringTeam
          (:NewEnumerator0
            (if (> _returnvalue_2 3) :!label _label_3
              (LocalVariables|SetProgressToAdd 3)
              (else
                (LocalVariables|SetProgressToAdd _returnvalue_2)))
            (if (> (+ (Variables|Default|GetProgress) (LocalVariables|GetProgressToAdd)) 100)
              (Variables|Default|SetProgress 100)
              (else
                (Variables|Default|SetProgress (+ (Variables|Default|GetProgress) (LocalVariables|GetProgressToAdd)))))
            (Variables|Default|SetOwningTeam "NewEnumerator0")
            (goto _label))
          (:NewEnumerator1
            (if (> _returnvalue_3 3) :!label _label_4
              (LocalVariables|SetProgressToAdd 3)
              (else
                (LocalVariables|SetProgressToAdd _returnvalue_3)))
            (if (> (+ (Variables|Default|GetProgress) (LocalVariables|GetProgressToAdd)) 100)
              (Variables|Default|SetProgress 100)
              (else
                (Variables|Default|SetProgress (+ (Variables|Default|GetProgress) (LocalVariables|GetProgressToAdd)))))
            (Variables|Default|SetOwningTeam "NewEnumerator1")
            (goto _label)))
        (elif (Utilities|Enum|Equal(Enum) (Variables|Default|GetOwningTeam) "NewEnumerator0")
          (if (Utilities|Enum|Equal(Enum) ScoringTeam "NewEnumerator0")
            (goto _label_3)
            (else
              (if (> _returnvalue_4 3)
                (LocalVariables|SetProgressToAdd 3)
                (else
                  (LocalVariables|SetProgressToAdd _returnvalue_4)))
              (if (< (- (Variables|Default|GetProgress) (LocalVariables|GetProgressToAdd)) 0)
                (Variables|Default|SetProgress 0)
                (Variables|Default|SetOwningTeam "NewEnumerator2")
                (goto _label)
                (else
                  (Variables|Default|SetProgress (- (Variables|Default|GetProgress) (LocalVariables|GetProgressToAdd)))
                  (Variables|Default|SetOwningTeam "NewEnumerator0")
                  (goto _label)))))
          (elif (Utilities|Enum|Equal(Enum) (Variables|Default|GetOwningTeam) "NewEnumerator1")
            (if (Utilities|Enum|Equal(Enum) ScoringTeam "NewEnumerator1")
              (goto _label_4)
              (else
                (if (> _returnvalue 3)
                  (LocalVariables|SetProgressToAdd 3)
                  (else
                    (LocalVariables|SetProgressToAdd _returnvalue)))
                (if (< (- (Variables|Default|GetProgress) (LocalVariables|GetProgressToAdd)) 0)
                  (Variables|Default|SetProgress 0)
                  (Variables|Default|SetOwningTeam "NewEnumerator2")
                  (goto _label)
                  (else
                    (Variables|Default|SetProgress (- (Variables|Default|GetProgress) (LocalVariables|GetProgressToAdd)))
                    (Variables|Default|SetOwningTeam "NewEnumerator1")
                    (goto _label)))))))))
    (:NewEnumerator1
      (goto _label_2))))