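; XP booster actor that players use via a timed multi-use entry to boost every living player pawn within its radius.
; Each pawn gains 115% of the XP gap to its next ExperienceRamp threshold, applied on the dedicated server.
; Use consumes the booster until server-side Activate re-enables it; replicated CanBeUsed toggles mesh and light visibility through its OnRep.
; Rings spin on Tick outside dedicated servers.
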(event EventTick
  (params (DeltaSeconds :type Float%20%28single-precision%29))
  (Utilities|TWDedicatedServerCheck
    (:No
      (Transformation|AddLocalRotation (Variables|Default|Getring1) "0.700000, 0,0.500000" false)
      (Transformation|AddLocalRotation (Variables|Default|Getring2) "0.300000,0.050000,-0.600000" false))))

(fn ConstructionScript
  (Components|Sphere|SetSphereRadius (Variables|Default|GetSphere1) (Variables|Default|GetRadius) true))

(fn BPGetMultiUseEntries
  (params (ForPC :type Player%20Controller%20Object%20Reference) (MultiUseEntries :type Array%20of%20Multi%20Use%20Entry%20Structures))
  (LocalVariables|SetUseEntries MultiUseEntries)
  (if (Variables|Default|GetCanBeUsed)
    (Utilities|Array|Add (LocalVariables|GetUseEntries) (Utilities|Struct|MakeMultiUseEntry 0 "Hold to apply XP boost to player around" 888 1 true false false false false false false "(B=175,G=175,R=175,A=255)" 0.0 0.0))
    (Utilities|Array|Add (LocalVariables|GetUseEntries) (Utilities|Struct|MakeMultiUseEntry 0 "Apply XP Boost" 999 0 false false false false false false false "(B=175,G=175,R=175,A=255)" 0.0 15.0)))
  (return (LocalVariables|GetUseEntries)))

(fn BPTryMultiUse
  (params (ForPC :type Player%20Controller%20Object%20Reference) (UseIndex :type Integer))
  (if (== UseIndex 999)
    (if (Variables|Default|GetCanBeUsed)
      (bind _astw_gamestate_c (Utilities|Casting|CastToTW_GameState (Game|GetGameState))
        (:then
          (bind _returnvalue (Class|ShooterGameState|BaseGetAllShooterCharacters _astw_gamestate_c))
          (for _array_element _returnvalue
            (bind _astw_playerpawntest_c (Utilities|Casting|CastToTW_PlayerPawnTest _array_element))
            (if (Class|PrimalCharacter|IsAlive _astw_playerpawntest_c)
              (bind _returnvalue_2 (Transformation|GetDistanceTo _astw_playerpawntest_c self))
              (if (< _returnvalue_2 (Variables|Default|GetRadius))
                (CallFunction|ApplyXPBoost _astw_playerpawntest_c))))
          (Variables|Default|SetCanBeUsed false)
          (Networking|ForceNetUpdate))
        (:CastFailed
          _)))
    (return false)))

(fn ApplyXPBoost
  (params (Pawn :type TW%20Player%20Pawn%20Test%20Object%20Reference))
  (bind _playercharacterstatus (Variables|/Game/PrimalEarth/CoreBlueprints/PlayerPawnTest.PlayerPawnTest_C|GetPlayerCharacterStatus Pawn))
  (Utilities|TWDedicatedServerCheck
    (:Yes
      (bind _astw_gamestate_c (Utilities|Casting|CastToTW_GameState (Game|GetGameState)))
      (bind (_array_element _array_index) (Utilities|Array|ForEachLoopwithBreak (Variables|/Game/Mods/TribeWars/TW_GameState.TW_GameState_C|GetExperienceRamp _astw_gamestate_c) :!label _label)
        (:LoopBody
          (if (> _array_element (Variables|/Script/ShooterGame.PrimalCharacterStatusComponent|GetExperiencePoints _playercharacterstatus))
            (Variables|/Script/ShooterGame.PrimalCharacterStatusComponent|SetExperiencePoints _playercharacterstatus (+ (* (- (Utilities|Array|Get(acopy) (Variables|/Game/Mods/TribeWars/TW_GameState.TW_GameState_C|GetExperienceRamp _astw_gamestate_c) _array_index) (Variables|/Script/ShooterGame.PrimalCharacterStatusComponent|GetExperiencePoints _playercharacterstatus)) 1.15) (Variables|/Script/ShooterGame.PrimalCharacterStatusComponent|GetExperiencePoints _playercharacterstatus)))
            (goto _label Break)))))))

(fn OnRepCanbeUsed
  (if (Variables|Default|GetCanBeUsed)
    (Development|SetHiddeninGame (Variables|Default|Getroot) false true)
    (Rendering|SetVisibility (Variables|Default|GetPointLight1) true false)
    (else
      (Development|SetHiddeninGame (Variables|Default|Getroot) true true)
      (Rendering|SetVisibility (Variables|Default|GetPointLight1) false false))))

(fn Activate
  (Utilities|TWDedicatedServerCheck
    (:Yes
      (Variables|Default|SetCanBeUsed true)
      (Networking|ForceNetUpdate))))

(fn Deactivate
  (Utilities|TWDedicatedServerCheck
    (:Yes
      (Variables|Default|SetCanBeUsed false)
      (Networking|ForceNetUpdate))))