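; Event spawner actor that, when activated on the dedicated server, spawns a random DinoEntries type at line-traced ground points within its sphere trigger.
; Replicated IsActive drives a client event marker widget, hidden while the local player is inside the trigger.
; CheckIfReady checks on the server that no living team player is within the radius.
; Deactivation clears the dino list without destroying dinos; per-dino markers are disconnected due to widget tick issues.
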(event OnComponentBeginOverlap(Trigger)
  (params (OtherActor :type Actor%20Object%20Reference) (OtherComp :type Primitive%20Component%20Object%20Reference) (OtherBodyIndex :type Integer) (bFromSweep :type Boolean) (SweepResult :type Hit%20Result%20Structure%20%28by%20ref%29))
  (if (Variables|Default|GetIsActive)
    (bind _astw_playerpawntest_c (Utilities|Casting|CastToTW_PlayerPawnTest OtherActor))
    (Utilities|TWDedicatedServerCheck
      (:No
        (if (Pawn|IsLocallyControlled _astw_playerpawntest_c)
          (bind _astw_playercontrollerblueprint_c (Utilities|Casting|CastToTW_PlayerControllerBlueprint (Pawn|GetController _astw_playerpawntest_c)))
          (CallFunction|RemoveEventMarker))))))

(event OnComponentEndOverlap(Trigger)
  (params (OtherActor :type Actor%20Object%20Reference) (OtherComp :type Primitive%20Component%20Object%20Reference) (OtherBodyIndex :type Integer))
  (if (Variables|Default|GetIsActive)
    (bind _astw_playerpawntest_c (Utilities|Casting|CastToTW_PlayerPawnTest OtherActor))
    (Utilities|TWDedicatedServerCheck
      (:No
        (if (Pawn|IsLocallyControlled _astw_playerpawntest_c)
          (bind _astw_playercontrollerblueprint_c (Utilities|Casting|CastToTW_PlayerControllerBlueprint (Pawn|GetController _astw_playerpawntest_c)))
          (CallFunction|CreateEventMarker _astw_playercontrollerblueprint_c))))))

(event Custom|ActivateDinoSpawner
  (Utilities|TWDedicatedServerCheck
    (:Yes
      (Variables|Default|SetIsActive true)
      (bind _dinotospawn (CallFunction|PickDinotoSpawn))
      (Variables|Default|SetChoosenDinoType _dinotospawn)
      (for _index (range 1 (.Amount (Utilities|Struct|BreakTW_DinoSpawnSelection_Struct _dinotospawn)))
        (bind _spawnpoint (CallFunction|FindDinoSpawnpoint))
        (bind _returnvalue (Class|PrimalDinoCharacter|SpawnDino (Class|Actor|GetWorld) (.DinoType (Utilities|Struct|BreakTW_DinoSpawnSelection_Struct _dinotospawn)) _spawnpoint "0, 0, 0" 1.0 0 false false 0 false 1.0 (Math|Random|RandomIntegerinRange 1 15)))
        (Utilities|Array|Add (Variables|Default|GetSpawnedDinos) _returnvalue))
      (Networking|ForceNetUpdate))))

(event Custom|DeactivateDinoSpawner
  (Utilities|TWDedicatedServerCheck
    (:Yes
      (Variables|Default|SetIsActive false)
      (Utilities|Array|Clear (Variables|Default|GetSpawnedDinos))
      (Networking|ForceNetUpdate))))

(event Custom|OnDied_Event
  (params (DiedCharacter :type Primal%20Character%20Object%20Reference))
  ;[1 1 1] dino markers unused due to weird widget tick behaviour
  (Development|PrintString "death")
  (CallFunction|RemoveDinoMarkers)
  (bind _astw_playercontrollerblueprint_c (Utilities|Casting|CastToTW_PlayerControllerBlueprint (Pawn|GetController DiedCharacter)))
  (CallFunction|CreateEventMarker _astw_playercontrollerblueprint_c))

(fn ConstructionScript
  (bind _trigger (Variables|Default|GetTrigger))
  (if (Variables|Default|GetIsDebugMode)
    (Components|Sphere|SetSphereRadius _trigger 2.5e+03 true)
    (else
      (Components|Sphere|SetSphereRadius _trigger 8e+03 true))))

(fn CreateDinoMarkers
  (params (Controller :type TW%20Player%20Controller%20Blueprint%20Object%20Reference) (Dino :type Actor%20Object%20Reference))
  (bind _returnvalue (UserInterface|CreateWidget "/Game/Mods/TribeWars/HUD/Events/TW_EventMarker_Widget.TW_EventMarker_Widget_C" Controller))
  (UserInterface|Viewport|AddtoViewport _returnvalue)
  (Utilities|Array|Add (Variables|Default|GetDinoMarkers) _returnvalue)
  (Variables|/Game/Mods/TribeWars/HUD/Events/TW_EventMarker_Widget.TW_EventMarker_Widget_C|SetMarkerActor _returnvalue Dino))

(fn RemoveDinoMarkers
  (bind _dinomarkers (Variables|Default|GetDinoMarkers))
  (for _array_element _dinomarkers
    (Utilities|IsValid _array_element
      (:Is%20Valid
        (Class|UserWidget|RemovefromViewport _array_element))))
  (Utilities|Array|Clear _dinomarkers))

(fn CreateEventMarker
  (params (Controller :type TW%20Player%20Controller%20Blueprint%20Object%20Reference))
  (bind _returnvalue (UserInterface|CreateWidget "/Game/Mods/TribeWars/HUD/Events/TW_EventMarker_Widget.TW_EventMarker_Widget_C" Controller))
  (UserInterface|Viewport|AddtoViewport _returnvalue)
  (Variables|Default|SetEventMarkerWidget _returnvalue)
  (Variables|/Game/Mods/TribeWars/HUD/Events/TW_EventMarker_Widget.TW_EventMarker_Widget_C|SetMarkerActor _returnvalue self)
  (Default|SetIcon _returnvalue "NewEnumerator2"))

(fn RemoveEventMarker
  (Utilities|IsValid (Variables|Default|GetEventMarkerWidget)
    (:Is%20Valid
      (Class|UserWidget|RemovefromViewport (Variables|Default|GetEventMarkerWidget))
      (Variables|Default|SetEventMarkerWidget 0))))

(fn OnRepIsActive
  (Utilities|TWDedicatedServerCheck
    (:No
      (if (Variables|Default|GetIsActive)
        (bind _astw_playercontrollerblueprint_c (Utilities|Casting|CastToTW_PlayerControllerBlueprint (Game|GetPlayerController 0)))
        (CallFunction|CreateEventMarker _astw_playercontrollerblueprint_c)
        (else
          (CallFunction|RemoveDinoMarkers)
          (CallFunction|RemoveEventMarker))))))

(fn CheckifReady
  (Utilities|TWDedicatedServerCheck
    (:Yes
      (if (Variables|Default|GetIsActive)
        _
        (else
          (bind _astw_gamestate_c (Utilities|Casting|CastToTW_GameState (Game|GetGameState))
            (:then
              (LocalVariables|SetLocalIsReady true)
              (for _array_element (Variables|/Game/Mods/TribeWars/TW_GameState.TW_GameState_C|GetRedTeam_PlayerData _astw_gamestate_c)
                (if (.IsAlive (Utilities|Struct|BreakTW_PlayerData _array_element))
                  (bind _astw_playerpawntest_c (Utilities|Casting|CastToTW_PlayerPawnTest (Pawn|GetControlledPawn (.Controller (Utilities|Struct|BreakTW_PlayerData _array_element)))))
                  (bind _returnvalue (Transformation|GetDistanceTo _astw_playerpawntest_c))
                  (if (not (> _returnvalue (Variables|/Script/Engine.SphereComponent|GetSphereRadius (Variables|Default|GetTrigger))))
                    (LocalVariables|SetLocalIsReady false))))
              (for _array_element_2 (Variables|/Game/Mods/TribeWars/TW_GameState.TW_GameState_C|GetBlueTeam_PlayerData _astw_gamestate_c)
                (if (.IsAlive (Utilities|Struct|BreakTW_PlayerData _array_element_2))
                  (bind _astw_playerpawntest_c_2 (Utilities|Casting|CastToTW_PlayerPawnTest (Pawn|GetControlledPawn (.Controller (Utilities|Struct|BreakTW_PlayerData _array_element_2)))))
                  (bind _returnvalue_2 (Transformation|GetDistanceTo _astw_playerpawntest_c_2))
                  (if (not (> _returnvalue_2 (Variables|/Script/Engine.SphereComponent|GetSphereRadius (Variables|Default|GetTrigger))))
                    (LocalVariables|SetLocalIsReady false)))))
            (:CastFailed
              _))))
      (return (LocalVariables|GetLocalIsReady)))))

(fn FindDinoSpawnpoint
  (bind _self self)
  (bind _returnvalue (Transformation|GetActorLocation _self))
  (LocalVariables|SetLocalRadius (Math|Random|RandomFloatinRange 5e+01 (Variables|/Script/Engine.SphereComponent|GetSphereRadius (Variables|Default|GetTrigger))))
  (LocalVariables|SetLocalAngle (* (* (Math|Random|RandomFloatinRange 0.0 1.0) 2.0) (Math|Trig|GetPI)))
  (bind _outhit (Collision|LineTraceByChannel (+ (Math|Vector|MakeVector (* (Math|Trig|Cos(Radians) (LocalVariables|GetLocalAngle)) (LocalVariables|GetLocalRadius)) (* (Math|Trig|Sin(Radians) (LocalVariables|GetLocalAngle)) (LocalVariables|GetLocalRadius)) 1.2e+04) (Math|Vector|MakeVector (.x _returnvalue) (.y _returnvalue) 0.0)) (+ (Math|Vector|MakeVector (* (Math|Trig|Cos(Radians) (LocalVariables|GetLocalAngle)) (LocalVariables|GetLocalRadius)) (* (Math|Trig|Sin(Radians) (LocalVariables|GetLocalAngle)) (LocalVariables|GetLocalRadius)) -1.5e+04) (Math|Vector|MakeVector (.x _returnvalue) (.y _returnvalue) 0.0)) "ECC_WorldStatic" false 0 "None"))
  (return (.Location (Collision|BreakHitResult _outhit))))

(fn PickDinotoSpawn
  (bind _dinoentries (Variables|Default|GetDinoEntries))
  (return (Utilities|Array|Get(acopy) _dinoentries (Math|Random|RandomIntegerinRange 0 (Utilities|Array|LastIndex _dinoentries)))))