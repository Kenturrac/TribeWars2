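; Event spawner that scatters TW_XPBooster pickups inside its Trigger sphere while active.
; The dedicated server activates and deactivates it, spawning boosters at random line-traced ground points and destroying them afterwards.
; Replicated IsActive drives a client-side event marker widget, which hides while the local player is inside the sphere.
; CheckIfReady reports whether the inactive spawner's radius is clear of living players from both teams.
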(event OnComponentBeginOverlap(Trigger)
  (params (OtherActor :type Actor%20Object%20Reference) (OtherComp :type Primitive%20Component%20Object%20Reference) (OtherBodyIndex :type Integer) (bFromSweep :type Boolean) (SweepResult :type Hit%20Result%20Structure%20%28by%20ref%29))
  (if (Variables|Default|GetIsActive)
    (bind _astw_playerpawntest_c (Utilities|Casting|CastToTW_PlayerPawnTest OtherActor))
    (Utilities|TWDedicatedServerCheck
      (:No
        (if (Pawn|IsLocallyControlled _astw_playerpawntest_c)
          (Utilities|Casting|CastToTW_PlayerControllerBlueprint (Pawn|GetController _astw_playerpawntest_c))
          (CallFunction|RemoveEventMarker))))))

(event OnComponentEndOverlap(Trigger)
  (params (OtherActor :type Actor%20Object%20Reference) (OtherComp :type Primitive%20Component%20Object%20Reference) (OtherBodyIndex :type Integer))
  (if (Variables|Default|GetIsActive)
    (bind _astw_playerpawntest_c (Utilities|Casting|CastToTW_PlayerPawnTest OtherActor))
    (Utilities|TWDedicatedServerCheck
      (:No
        (if (Pawn|IsLocallyControlled _astw_playerpawntest_c)
          (bind _astw_playercontrollerblueprint_c (Utilities|Casting|CastToTW_PlayerControllerBlueprint (Pawn|GetController _astw_playerpawntest_c)))
          (CallFunction|CreateEventMarker _astw_playercontrollerblueprint_c))))))

(event Custom|ActivateXPSpawner
  (Utilities|TWDedicatedServerCheck
    (:Yes
      (Variables|Default|SetIsActive true)
      (for _index (range 1 3)
        (bind _spawnpoint (CallFunction|FindSpawnpoint))
        (bind _returnvalue (Game|SpawnActorfromClass "/Game/Mods/TribeWars/Blueprints/CoreSystems/TW_XPBooster_BP.TW_XPBooster_BP_C" (Math|Transform|MakeTransform _spawnpoint "0, 0, 0" "1,1,1") false 0))
        (Default|Activate _returnvalue)
        (Utilities|Array|Add (Variables|Default|GetSpawnedXPBooster) _returnvalue))
      (Networking|ForceNetUpdate))))

(event Custom|DeactivateXPSpawner
  (bind _spawnedxpbooster (Variables|Default|GetSpawnedXPBooster))
  (Utilities|TWDedicatedServerCheck
    (:Yes
      (Variables|Default|SetIsActive false)
      (for _array_element _spawnedxpbooster
        (Actor|DestroyActor _array_element))
      (Utilities|Array|Clear _spawnedxpbooster)
      (Networking|ForceNetUpdate))))

(fn ConstructionScript
  (bind _trigger (Variables|Default|GetTrigger))
  (if (Variables|Default|GetIsDebugMode)
    (Components|Sphere|SetSphereRadius _trigger 6e+02 true)
    (else
      (Components|Sphere|SetSphereRadius _trigger 6e+03 true))))

(fn CreateEventMarker
  (params (Controller :type TW%20Player%20Controller%20Blueprint%20Object%20Reference))
  (bind _returnvalue (UserInterface|CreateWidget "/Game/Mods/TribeWars/HUD/Events/TW_EventMarker_Widget.TW_EventMarker_Widget_C" Controller))
  (UserInterface|Viewport|AddtoViewport _returnvalue)
  (Variables|Default|SetEventMarkerWidget _returnvalue)
  (Variables|/Game/Mods/TribeWars/HUD/Events/TW_EventMarker_Widget.TW_EventMarker_Widget_C|SetMarkerActor _returnvalue self)
  (Default|SetIcon _returnvalue "NewEnumerator1"))

(fn RemoveEventMarker
  (Utilities|IsValid (Variables|Default|GetEventMarkerWidget)
    (:Is%20Valid
      (Class|UserWidget|RemovefromViewport (Variables|Default|GetEventMarkerWidget))
      (Variables|Default|SetEventMarkerWidget 0))))

(fn OnRepIsActive
  (Utilities|TWDedicatedServerCheck
    (:No
      (if (Variables|Default|GetIsActive)
        (bind _astw_playercontrollerblueprint_c (Utilities|Casting|CastToTW_PlayerControllerBlueprint (Game|GetPlayerController 0)))
        (CallFunction|CreateEventMarker _astw_playercontrollerblueprint_c)
        (else
          (CallFunction|RemoveEventMarker))))))

(fn CheckifReady
  (Utilities|TWDedicatedServerCheck
    (:Yes
      (if (Variables|Default|GetIsActive)
        _
        (else
          (bind _astw_gamestate_c (Utilities|Casting|CastToTW_GameState (Game|GetGameState))
            (:then
              (LocalVariables|SetLocalIsReady true)
              (for _array_element (Variables|/Game/Mods/TribeWars/TW_GameState.TW_GameState_C|GetRedTeam_PlayerData _astw_gamestate_c)
                (if (.IsAlive (Utilities|Struct|BreakTW_PlayerData _array_element))
                  (bind _astw_playerpawntest_c (Utilities|Casting|CastToTW_PlayerPawnTest (Pawn|GetControlledPawn (.Controller (Utilities|Struct|BreakTW_PlayerData _array_element)))))
                  (bind _returnvalue (Transformation|GetDistanceTo _astw_playerpawntest_c))
                  (if (not (> _returnvalue (Variables|/Script/Engine.SphereComponent|GetSphereRadius (Variables|Default|GetTrigger))))
                    (LocalVariables|SetLocalIsReady false))))
              (for _array_element_2 (Variables|/Game/Mods/TribeWars/TW_GameState.TW_GameState_C|GetBlueTeam_PlayerData _astw_gamestate_c)
                (if (.IsAlive (Utilities|Struct|BreakTW_PlayerData _array_element_2))
                  (bind _astw_playerpawntest_c_2 (Utilities|Casting|CastToTW_PlayerPawnTest (Pawn|GetControlledPawn (.Controller (Utilities|Struct|BreakTW_PlayerData _array_element_2)))))
                  (bind _returnvalue_2 (Transformation|GetDistanceTo _astw_playerpawntest_c_2))
                  (if (not (> _returnvalue_2 (Variables|/Script/Engine.SphereComponent|GetSphereRadius (Variables|Default|GetTrigger))))
                    (LocalVariables|SetLocalIsReady false)))))
            (:CastFailed
              _))))
      (return (LocalVariables|GetLocalIsReady)))))

(fn FindSpawnpoint
  (bind _self self)
  (bind _returnvalue (Transformation|GetActorLocation _self))
  (LocalVariables|SetLocalRadius (Math|Random|RandomFloatinRange 5e+01 (Variables|/Script/Engine.SphereComponent|GetSphereRadius (Variables|Default|GetTrigger))))
  (LocalVariables|SetLocalAngle (* (* (Math|Random|RandomFloatinRange 0.0 1.0) 2.0) (Math|Trig|GetPI)))
  (bind _outhit (Collision|LineTraceByChannel (+ (Math|Vector|MakeVector (* (Math|Trig|Cos(Radians) (LocalVariables|GetLocalAngle)) (LocalVariables|GetLocalRadius)) (* (Math|Trig|Sin(Radians) (LocalVariables|GetLocalAngle)) (LocalVariables|GetLocalRadius)) 1.2e+04) (Math|Vector|MakeVector (.x _returnvalue) (.y _returnvalue) 0.0)) (+ (Math|Vector|MakeVector (* (Math|Trig|Cos(Radians) (LocalVariables|GetLocalAngle)) (LocalVariables|GetLocalRadius)) (* (Math|Trig|Sin(Radians) (LocalVariables|GetLocalAngle)) (LocalVariables|GetLocalRadius)) -1.5e+04) (Math|Vector|MakeVector (.x _returnvalue) (.y _returnvalue) 0.0)) "ECC_WorldDynamic" false 0 "None"))
  (return (+ (.Location (Collision|BreakHitResult _outhit)) "0, 0,100.000000")))