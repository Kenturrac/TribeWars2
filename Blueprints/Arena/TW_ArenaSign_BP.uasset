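; Arena sign actor that shows the name and kill count of the player with the most warm-up (pre-game) kills.
; A Delay on Tick throttles updates to roughly half-second intervals.
; During warm-up, the dedicated server scans all shooter controllers for a new highest PreGameKills, stores it and calls ForceNetUpdate.
; Non-dedicated instances write that leader's name and kills to eight text elements.
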(event EventTick
  (params (DeltaSeconds :type Float%20%28single-precision%29))
  (Utilities|FlowControl|Delay 0.5)
  (if (Networking|IsDedicatedServer)
    (bind _astw_gamestate_c (Utilities|Casting|CastToTW_GameState (Game|GetGameState)))
    (if (Variables|/Game/Mods/TribeWars/TW_GameState.TW_GameState_C|GetWarmUpState _astw_gamestate_c)
      (bind _returnvalue (Class|CustomGameState|GetAllShooterControllers _astw_gamestate_c))
      (for _array_element _returnvalue
        (bind _astw_playercontrollerblueprint_c (Utilities|Casting|CastToTW_PlayerControllerBlueprint _array_element))
        (if (> (Variables|/Game/Mods/TribeWars/TW_PlayerControllerBlueprint.TW_PlayerControllerBlueprint_C|GetPreGameKills _astw_playercontrollerblueprint_c) (Variables|Default|GetLocalCurrentHighestKills))
          (Variables|Default|SetLocalCurrentHighestKills (Variables|/Game/Mods/TribeWars/TW_PlayerControllerBlueprint.TW_PlayerControllerBlueprint_C|GetPreGameKills _astw_playercontrollerblueprint_c))
          (Variables|Default|SetLocalCurrentHighestKillsPlayerName (Variables|/Game/Mods/TribeWars/TW_PlayerControllerBlueprint.TW_PlayerControllerBlueprint_C|GetPlayerName _astw_playercontrollerblueprint_c))
          (Development|PrintString "Hello")))
      (if (> (Variables|Default|GetLocalCurrentHighestKills) 0)
        (Variables|Default|SetCurrentHighestKills (Variables|Default|GetLocalCurrentHighestKills))
        (Variables|Default|SetCurrentHighestKillsPlayerName (Variables|Default|GetLocalCurrentHighestKillsPlayerName))
        (Networking|ForceNetUpdate)))
    (elif (and (> (Variables|Default|GetCurrentHighestKills) 0) (Utilities|Enum|NotEqual(Enum) (Variables|Default|GetCurrentHighestKillsPlayerName) ""))
      (Rendering|Components|TextRender|SetText (Variables|Default|Geta1) (Utilities|String|Append (Utilities|String|Append (Utilities|String|Append (Variables|Default|GetCurrentHighestKillsPlayerName) " - ") (Utilities|String|ToString(Integer) (Variables|Default|GetCurrentHighestKills))) " kills")))))

(fn ConstructionScript)