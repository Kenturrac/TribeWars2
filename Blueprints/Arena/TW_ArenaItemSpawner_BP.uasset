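; Arena weapon spawner that offers a random weapon, shield or grenade pickup through the multi-use menu and respawns it after a countdown.
; The dedicated server rolls WeaponIndex, whose RepNotify shows the matching rotating mesh and sets the light green, or red when empty.
; Using it adds the equipped item and any ammo to the player's inventory, then clears the index.
; Clearing starts the server countdown, replicated to text displays, which rerolls at zero.
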(event Custom|StartCountdown
  (Networking|SwitchHasAuthority
    (:Authority
      (Variables|Default|SetTimeCounter 15)
      (if (>= (Variables|Default|GetTimeCounter) 0) :!label _label
        (Utilities|FlowControl|Sequence
          (:then_0
            (Utilities|FlowControl|Delay 1.0)
            (Variables|Default|SetTimeCounter (- (Variables|Default|GetTimeCounter) 1))
            (Networking|ForceNetUpdate)
            (goto _label))
          (:then_1
            (if (== (Variables|Default|GetTimeCounter) 0)
              (CallFunction|ActivatePickup))))))))

(event EventTick
  (params (DeltaSeconds :type Float%20%28single-precision%29))
  (if (not (Networking|IsDedicatedServer))
    (Transformation|AddLocalRotation (Variables|Default|GetRotator) "0,1.000000, 0" false)))

(event EventBeginPlay
  (CallFunction|ActivatePickup))

(fn ConstructionScript)

(fn BPGetMultiUseEntries
  (params (ForPC :type Player%20Controller%20Object%20Reference) (MultiUseEntries :type Array%20of%20Multi%20Use%20Entry%20Structures))
  (LocalVariables|SetReturnUseEntries MultiUseEntries)
  (if (> (Variables|Default|GetWeaponIndex) 0)
    (Utilities|Array|Add (LocalVariables|GetReturnUseEntries) (Utilities|Struct|MakeMultiUseEntry 0 "Pick up weapon" 1 0 false false false true)))
  (return (LocalVariables|GetReturnUseEntries)))

(fn BPTryMultiUse
  (params (ForPC :type Player%20Controller%20Object%20Reference) (UseIndex :type Integer))
  (bind _asplayerpawntest_c (Utilities|Casting|CastToPlayerPawnTest (Pawn|GetControlledPawn ForPC)))
  (switch int UseIndex
    (:1
      (Variables|/Script/ShooterGame.PrimalInventoryComponent|SetbReceivingEquippedItems (Variables|/Game/PrimalEarth/CoreBlueprints/PlayerPawnTest.PlayerPawnTest_C|GetPrimalInventory1 _asplayerpawntest_c) true)
      (switch int (Variables|Default|GetWeaponIndex)
        (:1
          (Class|PrimalItem|AddNewItem "/Game/PrimalEarth/CoreBlueprints/Weapons/PrimalItem_GasGrenade.PrimalItem_GasGrenade_C" (Variables|/Game/PrimalEarth/CoreBlueprints/PlayerPawnTest.PlayerPawnTest_C|GetPrimalInventory1 _asplayerpawntest_c) true false 0.0 false 2 false))
        (:2
          (Class|PrimalItem|AddNewItem "/Game/PrimalEarth/CoreBlueprints/Weapons/PrimalItem_WeaponGrenade.PrimalItem_WeaponGrenade_C" (Variables|/Game/PrimalEarth/CoreBlueprints/PlayerPawnTest.PlayerPawnTest_C|GetPrimalInventory1 _asplayerpawntest_c) true false 0.0 false 2 false))
        (:3
          (Class|PrimalItem|AddNewItem "/Game/PrimalEarth/CoreBlueprints/Items/Armor/Shields/PrimalItemArmor_MetalShield.PrimalItemArmor_MetalShield_C" (Variables|/Game/PrimalEarth/CoreBlueprints/PlayerPawnTest.PlayerPawnTest_C|GetPrimalInventory1 _asplayerpawntest_c) true false 0.0 false 1 false))
        (:4
          (Class|PrimalItem|AddNewItem "/Game/PrimalEarth/CoreBlueprints/Weapons/PrimalItem_WeaponBow.PrimalItem_WeaponBow_C" (Variables|/Game/PrimalEarth/CoreBlueprints/PlayerPawnTest.PlayerPawnTest_C|GetPrimalInventory1 _asplayerpawntest_c) true false 0.0 false 1 false)
          (Class|PrimalItem|AddNewItem "/Game/PrimalEarth/CoreBlueprints/Weapons/PrimalItemAmmo_ArrowStone.PrimalItemAmmo_ArrowStone_C" (Variables|/Game/PrimalEarth/CoreBlueprints/PlayerPawnTest.PlayerPawnTest_C|GetPrimalInventory1 _asplayerpawntest_c) false false 0.0 false 7 false))
        (:5
          (Class|PrimalItem|AddNewItem "/Game/PrimalEarth/CoreBlueprints/Weapons/PrimalItem_WeaponCrossbow.PrimalItem_WeaponCrossbow_C" (Variables|/Game/PrimalEarth/CoreBlueprints/PlayerPawnTest.PlayerPawnTest_C|GetPrimalInventory1 _asplayerpawntest_c) true false 0.0 false 1 false)
          (Class|PrimalItem|AddNewItem "/Game/PrimalEarth/CoreBlueprints/Weapons/PrimalItemAmmo_ArrowStone.PrimalItemAmmo_ArrowStone_C" (Variables|/Game/PrimalEarth/CoreBlueprints/PlayerPawnTest.PlayerPawnTest_C|GetPrimalInventory1 _asplayerpawntest_c) false false 0.0 false 5 false))
        (:6
          (Class|PrimalItem|AddNewItem "/Game/PrimalEarth/CoreBlueprints/Weapons/PrimalItem_WeaponShotgun.PrimalItem_WeaponShotgun_C" (Variables|/Game/PrimalEarth/CoreBlueprints/PlayerPawnTest.PlayerPawnTest_C|GetPrimalInventory1 _asplayerpawntest_c) true false 0.0 false 1 false)
          (Class|PrimalItem|AddNewItem "/Game/PrimalEarth/CoreBlueprints/Weapons/PrimalItemAmmo_SimpleShotgunBullet.PrimalItemAmmo_SimpleShotgunBullet_C" (Variables|/Game/PrimalEarth/CoreBlueprints/PlayerPawnTest.PlayerPawnTest_C|GetPrimalInventory1 _asplayerpawntest_c) false false 0.0 false 6 false))
        (:7
          (Class|PrimalItem|AddNewItem "/Game/PrimalEarth/CoreBlueprints/Weapons/PrimalItem_WeaponOneShotRifle.PrimalItem_WeaponOneShotRifle_C" (Variables|/Game/PrimalEarth/CoreBlueprints/PlayerPawnTest.PlayerPawnTest_C|GetPrimalInventory1 _asplayerpawntest_c) true false 0.0 false 1 false)
          (Class|PrimalItem|AddNewItem "/Game/PrimalEarth/CoreBlueprints/Weapons/PrimalItemAmmo_SimpleRifleBullet.PrimalItemAmmo_SimpleRifleBullet_C" (Variables|/Game/PrimalEarth/CoreBlueprints/PlayerPawnTest.PlayerPawnTest_C|GetPrimalInventory1 _asplayerpawntest_c) false false 0.0 false 6 false))
        (:8
          (Class|PrimalItem|AddNewItem "/Game/PrimalEarth/CoreBlueprints/Weapons/PrimalItem_WeaponMachinedPistol.PrimalItem_WeaponMachinedPistol_C" (Variables|/Game/PrimalEarth/CoreBlueprints/PlayerPawnTest.PlayerPawnTest_C|GetPrimalInventory1 _asplayerpawntest_c) true false 0.0 false 1 false)
          (Class|PrimalItem|AddNewItem "/Game/PrimalEarth/CoreBlueprints/Weapons/PrimalItemAmmo_AdvancedBullet.PrimalItemAmmo_AdvancedBullet_C" (Variables|/Game/PrimalEarth/CoreBlueprints/PlayerPawnTest.PlayerPawnTest_C|GetPrimalInventory1 _asplayerpawntest_c) false false 0.0 false 5 false))
        (:9
          (Class|PrimalItem|AddNewItem "/Game/PrimalEarth/CoreBlueprints/Weapons/PrimalItem_WeaponSword.PrimalItem_WeaponSword_C" (Variables|/Game/PrimalEarth/CoreBlueprints/PlayerPawnTest.PlayerPawnTest_C|GetPrimalInventory1 _asplayerpawntest_c) true false 0.0 false 1 false))
        (:10
          (Class|PrimalItem|AddNewItem "/Game/PrimalEarth/CoreBlueprints/Weapons/PrimalItem_WeaponSpear.PrimalItem_WeaponSpear_C" (Variables|/Game/PrimalEarth/CoreBlueprints/PlayerPawnTest.PlayerPawnTest_C|GetPrimalInventory1 _asplayerpawntest_c) true false 0.0 false 3 false)))
      (Variables|Default|SetWeaponIndex 0)
      (Networking|ForceNetUpdate)
      (return true))))

(fn OnRepWeaponIndex
  (Development|SetHiddeninGame (Variables|Default|GetRotator) true true)
  (switch int (Variables|Default|GetWeaponIndex)
    (:0
      (Rendering|Components|Light|SetLightColor (Variables|Default|GetSpotLight1) "(R=1.000000,G=0.000000,B=0.000000,A=1.000000)")
      (Rendering|Material|SetMaterial (Variables|Default|GetBase_SMC) 1 "/Game/Mods/TribeWars/Materials/Instances/M_Utility_Light_3_Inst.M_Utility_Light_3_Inst")
      (if (Networking|IsDedicatedServer)
        (CallFunction|StartCountdown)))
    (:1
      (Development|SetHiddeninGame (Variables|Default|GetGasgrenade) false false)
      (Rendering|Components|Light|SetLightColor (Variables|Default|GetSpotLight1) "(R=0.000000,G=1.000000,B=0.000000,A=1.000000)" :!label _label)
      (Rendering|Material|SetMaterial (Variables|Default|GetBase_SMC) 1 "/Game/Mods/TribeWars/Materials/Instances/M_Utility_Light_2_Inst.M_Utility_Light_2_Inst"))
    (:2
      (Development|SetHiddeninGame (Variables|Default|GetGrenade) false false)
      (goto _label))
    (:3
      (Development|SetHiddeninGame (Variables|Default|GetShield) false false)
      (goto _label))
    (:4
      (Development|SetHiddeninGame (Variables|Default|GetBow) false false)
      (goto _label))
    (:5
      (Development|SetHiddeninGame (Variables|Default|GetCrossbow) false false)
      (goto _label))
    (:6
      (Development|SetHiddeninGame (Variables|Default|GetShotgun) false false)
      (goto _label))
    (:7
      (Development|SetHiddeninGame (Variables|Default|GetRifle) false false)
      (goto _label))
    (:8
      (Development|SetHiddeninGame (Variables|Default|GetPistol) false false)
      (goto _label))
    (:9
      (Development|SetHiddeninGame (Variables|Default|GetSword) false false)
      (goto _label))
    (:10
      (Development|SetHiddeninGame (Variables|Default|GetSpear) false false)
      (goto _label))))

(fn ActivatePickup
  (if (Networking|IsDedicatedServer)
    (Variables|Default|SetWeaponIndex (Math|Random|RandomIntegerinRange 1 10))
    (Networking|ForceNetUpdate)))

(fn DeactivatePickup
  (if (Networking|IsDedicatedServer)
    (Variables|Default|SetWeaponIndex 0)))

(fn OnRepTimeCounter
  (bind _textrender1 (Variables|Default|GetTextRender1))
  (Rendering|Components|TextRender|SetText (Variables|Default|GetTextRender1) (Utilities|String|ToString(Integer) (Variables|Default|GetTimeCounter)))
  (if (> (Variables|Default|GetTimeCounter) 0)
    (Development|SetHiddeninGame _textrender1 false false)
    (else
      (Development|SetHiddeninGame _textrender1 true false))))