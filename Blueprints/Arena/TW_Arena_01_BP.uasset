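; Arena Blueprint that outfits players with chitin armor when they enter its trigger during the warm-up state.
; It caches the TW game state on BeginPlay and handles trigger overlaps only on a dedicated server.
; A player pawn not yet flagged as in the start arena gets flagged, then receives a full, auto-equipped chitin set in its inventory, so the flag guards against repeat grants.
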(event OnActorBeginOverlap(Trigger)
  (params (OtherActor :type Actor%20Object%20Reference))
  (bind _mygamestate (Variables|Default|GetMyGameState))
  (if (Networking|IsDedicatedServer)
    (Utilities|IsValid _mygamestate
      (:Is%20Valid
        (if (Variables|/Game/Mods/TribeWars/TW_GameState.TW_GameState_C|GetWarmUpState _mygamestate)
          (bind _astw_playerpawntest_c (Utilities|Casting|CastToTW_PlayerPawnTest OtherActor))
          (if (not (Variables|/Game/Mods/TribeWars/TW_PlayerPawnTest.TW_PlayerPawnTest_C|GetIsInStartArena _astw_playerpawntest_c))
            (Variables|/Game/Mods/TribeWars/TW_PlayerPawnTest.TW_PlayerPawnTest_C|SetIsInStartArena _astw_playerpawntest_c true)
            (Class|PrimalItem|AddNewItem "/Game/PrimalEarth/CoreBlueprints/Items/Armor/Chitin/PrimalItemArmor_ChitinHelmet.PrimalItemArmor_ChitinHelmet_C" (Variables|/Game/PrimalEarth/CoreBlueprints/PlayerPawnTest.PlayerPawnTest_C|GetPrimalInventory1 _astw_playerpawntest_c) true false 0.0 false 1 false)
            (Class|PrimalItem|AddNewItem "/Game/PrimalEarth/CoreBlueprints/Items/Armor/Chitin/PrimalItemArmor_ChitinShirt.PrimalItemArmor_ChitinShirt_C" (Variables|/Game/PrimalEarth/CoreBlueprints/PlayerPawnTest.PlayerPawnTest_C|GetPrimalInventory1 _astw_playerpawntest_c) true false 0.0 false 1 false)
            (Class|PrimalItem|AddNewItem "/Game/PrimalEarth/CoreBlueprints/Items/Armor/Chitin/PrimalItemArmor_ChitinGloves.PrimalItemArmor_ChitinGloves_C" (Variables|/Game/PrimalEarth/CoreBlueprints/PlayerPawnTest.PlayerPawnTest_C|GetPrimalInventory1 _astw_playerpawntest_c) true false 0.0 false 1 false)
            (Class|PrimalItem|AddNewItem "/Game/PrimalEarth/CoreBlueprints/Items/Armor/Chitin/PrimalItemArmor_ChitinPants.PrimalItemArmor_ChitinPants_C" (Variables|/Game/PrimalEarth/CoreBlueprints/PlayerPawnTest.PlayerPawnTest_C|GetPrimalInventory1 _astw_playerpawntest_c) true false 0.0 false 1 false)
            (Class|PrimalItem|AddNewItem "/Game/PrimalEarth/CoreBlueprints/Items/Armor/Chitin/PrimalItemArmor_ChitinBoots.PrimalItemArmor_ChitinBoots_C" (Variables|/Game/PrimalEarth/CoreBlueprints/PlayerPawnTest.PlayerPawnTest_C|GetPrimalInventory1 _astw_playerpawntest_c) true false 0.0 false 1 false)))))))

(event EventBeginPlay
  (bind _astw_gamestate_c (Utilities|Casting|CastToTW_GameState (Game|GetGameState)))
  (Variables|Default|SetMyGameState _astw_gamestate_c))

(fn ConstructionScript)